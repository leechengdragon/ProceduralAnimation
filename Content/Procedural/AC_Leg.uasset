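; Procedural leg actor that walks on its parent body and can be thrown loose by physics, then crawl back and reattach.
; Control Rig's pre-forward solve dispatches by move style, driving the foot control with interpolation.
; Bind steps to traced plant points past a distance threshold, halved on first step to stagger legs.
; Free alternately anchors root and foot to inchworm toward the socket; Snap aligns both, reattaches and notifies the parent.
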(event `self.ControlRig.OnPreInitializeDelegate`
  (params (Component :type "ControlRigComponent Object Reference"))
  ;[0.05098 0.05098 0.05098] ControlRig相关逻辑
  ;;[0.05098 0.05098 0.05098] ControlRig初始化
  (`ControlRigComponent.AddMappedCompleteSkeletalMesh` Component (`self.Leg`)))

(event `self.ControlRig.OnPreForwardsSolveDelegate`
  (params (Component :type "ControlRigComponent Object Reference"))
  ;[0.05098 0.05098 0.05098] ControlRig相关逻辑
  ;;[0.05098 0.05098 0.05098] ControlRig前向解算
  (switch `/Game/Procedural/GameData/LegMoveStyle` (`self.MoveStyle`)
    (:`NewEnumerator0`
      (`self.HandleBindMove`))
    (:`NewEnumerator1`
      (`self.HandleFreeMove`))
    (:`NewEnumerator2`
      (`self.Handle Snap Move`))))

(event `BeginMoveToBody`
  (params (BodyPosition :type "Vector Structure"))
  ;[0.05098 0.05098 0.05098] 自定义事件
  ;;[0.05098 0.05098 0.05098] 向身体移动
  (`self.Init Free Move` BodyPosition))

(event `self.ReceiveBeginPlay`
  ;[0.05098 0.05098 0.05098] 初始化逻辑
  (`self.CalcLegLength`)
  ;;[0.05098 0.05098 0.05098] 初始化配置
  (`self.InitBindMoveConfig`)
  (`self.InitFreeMoveConfig`)
  (`self.ChangeMoveStyle` "NewEnumerator0")
  ;;[0.05098 0.05098 0.05098] 根据是否第一次迈腿确定范围超出距离
  (bind _over_range_distance (`self.HandleFirstStep`))
  (set `self.Bind_OverRangeDistance` _over_range_distance))

(event `self.ReceiveTick`
  (params (DeltaSeconds :type "Float (single-precision)"))
  ;[0.05098 0.05098 0.05098] Tick逻辑
  (set `self.Delta Seconds` DeltaSeconds)
  (switch `/Game/Procedural/GameData/LegMoveStyle` (`self.MoveStyle`)
    (:`NewEnumerator1`
      (`self.UpdateFreeMoveDirection`))))

(fn `Calc Plant Pos`
  (params (RootBone :type Name) (TraceOffset :type "Float (double-precision)") (TraceDistance :type "Float (double-precision)"))
  (returns (ResultPosition :type "Vector Structure"))
  (locals (TraceStartPosition :type "Vector Structure") (TraceEndPosition :type "Vector Structure"))
  ;[0.05098 0.05098 0.05098] 计算落脚点
  (`|ExecutionSequence`
    (:`then_0`
      ;;[0.05098 0.05098 0.05098] Step1:计算射线检测起点
      (bind _sockettransform (`self.Get Bind Socket Transform`))
      (set `local.TraceStartPosition` (+ (* (`KismetMathLibrary.GetForwardVector` (.rotation _sockettransform)) (`local.TraceOffset`)) (`SceneComponent.GetSocketLocation` (`self.Leg`) (`local.RootBone`)))))
    (:`then_1`
      ;;[0.05098 0.05098 0.05098] Step2:计算射线检测终点
      (set `local.TraceEndPosition` (+ (`local.TraceStartPosition`) (* (`KismetMathLibrary.Vector_Down`) (`local.TraceDistance`)))))
    (:`then_2`
      ;;[0.05098 0.05098 0.05098] Step3:向下进行射线检测，确定落脚点，如果没有检测到，则返回上一次落脚点
      (bind (_outhit _returnvalue) (`KismetSystemLibrary.LineTraceSingle` :`Start` (`local.TraceStartPosition`) :`End` (`local.TraceEndPosition`) :`TraceChannel` "TraceTypeQuery1" :`DrawDebugType` "ForOneFrame"))
      (if _returnvalue
        (return (`.Location` (`GameplayStatics.BreakHitResult` _outhit)))
        (else
          (return (`self.Bind_PlantTargetPosition`)))))))

(fn `CalcLegLength`
  (bind _leg (`self.Leg`))
  (bind _returnvalue (`SceneComponent.GetSocketLocation` _leg "Bone_001"))
  (bind _returnvalue_2 (`SceneComponent.GetSocketLocation` _leg "Bone_002"))
  (set `self.TotalLengthOfLeg` (+ (`KismetMathLibrary.Vector_Distance` (`SceneComponent.GetSocketLocation` _leg "Bone") _returnvalue) (`KismetMathLibrary.Vector_Distance` _returnvalue _returnvalue_2) (`KismetMathLibrary.Vector_Distance` _returnvalue_2 (`SceneComponent.GetSocketLocation` _leg "Bone_002_end")))))

(fn `Change Free Move Lock Bone`
  (params (IsLockEnd :type Boolean) (MoveDirectionNormal :type "Vector Structure") (UpTraceOffset :type "Float (double-precision)") (DownTraceOffset :type "Float (double-precision)"))
  (returns (LockPosition :type "Vector Structure") (MovePosition :type "Vector Structure"))
  (locals (RootBonePosition :type "Vector Structure" :default (0.0 0.0 0.0)) (LockTargetPosition :type "Vector Structure" :default (0.0 0.0 0.0)) (MoveTargetPosition :type "Vector Structure" :default (0.0 0.0 0.0)))
  (set `self.Free_IsLockEnd` (`local.IsLockEnd`))
  ;[0.05098 0.05098 0.05098] 缓存根骨骼位置
  (set `local.RootBonePosition` (`SceneComponent.GetSocketLocation` (`self.Leg`) (`self.RootBoneName`)))
  (`|ExecutionSequence`
    (:`then_0`
      (if (`local.IsLockEnd`)
        ;[0.05098 0.05098 0.05098] 锁定末端骨骼，移动根骨骼
        (`|ExecutionSequence`
          (:`then_0`
            ;;[0.05098 0.05098 0.05098] 计算锁定目标点
            (bind _hitposition (`self.DoLegTrace` (`SceneComponent.GetSocketLocation` (`self.Leg`) (`self.EndBoneName`)) (`local.UpTraceOffset`) (`local.DownTraceOffset`)))
            (set `local.LockTargetPosition` _hitposition))
          (:`then_1`
            ;;[0.05098 0.05098 0.05098] 计算移动目标点
            (bind _hitposition_2 (`self.DoLegTrace` (`self.CalcFreeMoveEntryPosition` (`local.RootBonePosition`) (`local.MoveDirectionNormal`) (* (`self.TotalLengthOfLeg`) (`self.Cfg_Free_MinMoveDistanceRatio`))) (`local.UpTraceOffset`) (`local.DownTraceOffset`)))
            (set `local.MoveTargetPosition` _hitposition_2)))
        (else
          ;[0.05098 0.05098 0.05098] 锁定根骨骼，移动末端骨骼
          (`|ExecutionSequence`
            (:`then_0`
              ;;[0.05098 0.05098 0.05098] 当锁定根骨骼的时候，锁定位置就是根骨骼位置
              (set `local.LockTargetPosition` (`local.RootBonePosition`)))
            (:`then_1`
              ;;[0.05098 0.05098 0.05098] 计算移动目标点
              (bind _hitposition_3 (`self.DoLegTrace` (`self.CalcFreeMoveEntryPosition` (`local.RootBonePosition`) (`local.MoveDirectionNormal`) (* (`self.TotalLengthOfLeg`) (`self.Cfg_Free_MaxMoveDistanceRatio`))) (`local.UpTraceOffset`) (`local.DownTraceOffset`)))
              (set `local.MoveTargetPosition` _hitposition_3))))))
    (:`then_1`
      (return (`local.LockTargetPosition`) (`local.MoveTargetPosition`)))))

(fn `ChangeMoveStyle`
  (params (MoveStyle :type "/Game/Procedural/GameData/LegMoveStyle Enum" :default "NewEnumerator0"))
  (bind _output_get (set `self.MoveStyle` MoveStyle))
  (`KismetSystemLibrary.PrintString` (`KismetStringLibrary.Concat_StrStr` "Change Move Style To " (`|GetEnumeratorNameAsString` _output_get)))
  (switch `/Game/Procedural/GameData/LegMoveStyle` (`self.MoveStyle`)
    (:`NewEnumerator0`
      (bind _resultposition (`self.Calc Plant Pos` (`self.RootBoneName`) (`self.Cfg_Bind_TraceOffset`) (`self.Cfg_Bind_TraceDistance`)))
      (set `self.Bind_PlantTargetPosition` _resultposition))))

(fn `CheckIsFreeMoveNearBindSocket`
  (returns (IsNearly :type Boolean))
  (bind _sockettransform (`self.Get Bind Socket Transform`))
  (return (<= (`KismetMathLibrary.Vector_Distance` (.location _sockettransform) (`SceneComponent.GetSocketLocation` (`self.Leg`) (`self.EndBoneName`))) (* (`self.TotalLengthOfLeg`) 0.5))))

(fn `CheckIsPlantPositionOverRange`
  (params (Position1 :type "Vector Structure") (Position2 :type "Vector Structure") (OverRangeDistance :type "Float (double-precision)"))
  (returns (IsOverRange :type Boolean))
  (bind (_position1_x _position1_y) (`KismetMathLibrary.BreakVector` (`local.Position1`)))
  (bind (_position2_x _position2_y) (`KismetMathLibrary.BreakVector` (`local.Position2`)))
  ;[1 1 1] 检测两点是否超过显示范围
  (return (> (`KismetMathLibrary.Vector_Distance` (`KismetMathLibrary.MakeVector` _position1_x _position1_y) (`KismetMathLibrary.MakeVector` _position2_x _position2_y)) (`local.OverRangeDistance`))))

(fn `Deactive Physic`
  (bind _leg (`self.Leg`))
  (`ActorComponent.SetActive` (`self.ControlRig`) true false)
  (`PrimitiveComponent.SetSimulatePhysics` _leg false)
  (`SkeletalMeshComponent.SetAllBodiesSimulatePhysics` _leg false)
  (`SkeletalMeshComponent.SetAllBodiesPhysicsBlendWeight` _leg 0.0 false))

(fn `DoLegTrace`
  (params (EntryPosition :type "Vector Structure") (UpTraceOffset :type "Float (double-precision)") (DownTraceOffset :type "Float (double-precision)"))
  (returns (HitPosition :type "Vector Structure"))
  (bind (_outhit _returnvalue) (`KismetSystemLibrary.LineTraceSingle` (+ (`local.EntryPosition`) (* (`KismetMathLibrary.Vector_Up`) (`local.UpTraceOffset`))) (+ (`local.EntryPosition`) (* (`KismetMathLibrary.Vector_Down`) (`local.DownTraceOffset`))) "TraceTypeQuery1"))
  (if _returnvalue
    (return (`.Location` (`GameplayStatics.BreakHitResult` _outhit)))))

(fn `FnishMoveToBody`
  (`self.ReCombineLeg`)
  (`self.ChangeMoveStyle` "NewEnumerator0")
  (`/Game/Procedural/BP_ProceduralMonster.SingleLimbFinishCombie` (`self.ParentReference`)))

(fn `Get Bind Socket Transform`
  (returns (SocketTransform :type "Transform Structure"))
  (return (`SceneComponent.GetSocketTransform` (`Character.Mesh` (`self.ParentReference`)) (`self.BindSocketName`) "RTS_World")))

(fn `Handle Snap Move`
  (locals (BindSocketPosition :type "Vector Structure" :default (0.0 0.0 0.0)) (IsRootBoneMoveFinished :type Boolean))
  (`|ExecutionSequence`
    (:`then_0`
      (bind _sockettransform (`self.Get Bind Socket Transform`))
      (set `local.BindSocketPosition` (.location _sockettransform)))
    (:`then_1`
      (bind _output_get (set `local.IsRootBoneMoveFinished` (`self.CheckIsAlreadyMoveToTarget` (`self.K2_GetActorLocation`) (`local.BindSocketPosition`))))
      (if _output_get
        (bind _resultposition (`self.Calc Plant Pos` "Bone" 220.0 600.0))
        (if (`self.CheckIsAlreadyMoveToTarget` (`SceneComponent.GetSocketLocation` (`self.Leg`) "Bone_002_end") _resultposition)
          (`self.FnishMoveToBody`)
          (else
            (bind _returnvalue (`self.LerpEndBonePosition` 5.0 _resultposition))
            (`ControlRigComponent.SetControlPosition` (`self.ControlRig`) "Bone_002_end_ctrl" _returnvalue "LocalSpace")))
        (else
          (bind _returnvalue_2 (`self.LerpRootBonePosition` 5.0 (`local.BindSocketPosition`)))
          (`self.K2_SetActorLocation` _returnvalue_2))))))

(fn `HandleBindMove`
  ;[0.05098 0.05098 0.05098] 绑定移动处理
  (`|ExecutionSequence`
    (:`then_0`
      ;;[0.05098 0.05098 0.05098] 实时计算落脚点
      (bind _resultposition (`self.Calc Plant Pos` (`self.RootBoneName`) (`self.Cfg_Bind_TraceOffset`) (`self.Cfg_Bind_TraceDistance`)))
      (set `self.Bind_PlantTracePosition` _resultposition))
    (:`then_1`
      ;;[0.05098 0.05098 0.05098] 检测当前落脚点与上次落脚点是否超过预定距离，如果超过则更新目标落脚点位置
      (bind _isoverrange (`self.CheckIsPlantPositionOverRange` (`self.Bind_PlantTracePosition`) (`self.Bind_PlantTargetPosition`) (`self.Bind_OverRangeDistance`)))
      (if _isoverrange
        (set `self.Bind_PlantTargetPosition` (`self.Bind_PlantTracePosition`))
        ;;[0.05098 0.05098 0.05098] 第一步迈腿的那条腿首次迈出后更新最大范围
        (if (`self.IsFirstStep`)
          (set `self.Bind_OverRangeDistance` (`self.Cfg_Bind_LegOverRangeDistance`)))))
    (:`then_2`
      ;;[0.05098 0.05098 0.05098] 当前落脚点和目标落脚点之间进行插值，并将位置设置给control rig 控制点
      (set `self.Bind_PlantPosition` (`KismetMathLibrary.VInterpTo` (`self.Bind_PlantPosition`) (`self.Bind_PlantTargetPosition`) (`self.Delta Seconds`) (`self.Cfg_Bind_LegLerpSpeed`)))
      (`ControlRigComponent.SetControlPosition` (`self.ControlRig`) "Bone_002_end_ctrl" (`self.Bind_PlantPosition`) "LocalSpace"))))

(fn `HandleFirstStep`
  (returns (`Over Range Distance` :type "Float (double-precision)"))
  ;[0.05098 0.05098 0.05098] 第一步跨出的腿目标距离为预定距离的一半，为了制作出交叉腿移动的效果
  (if (`self.IsFirstStep`)
    (return (* (`self.Cfg_Bind_LegOverRangeDistance`) 0.5))
    (else
      (return (`self.Cfg_Bind_LegOverRangeDistance`)))))

(fn `HandleFreeMove`
  (bind _isnearly (`self.CheckIsFreeMoveNearBindSocket`))
  (if _isnearly
    (`self.Init Snap Move`)
    (elif (`self.Free_IsLockEnd`)
      ;[0.05098 0.05098 0.05098] 锁定末端骨骼，移动根骨骼的处理，移动根骨骼相当与移动actor的位置，实际没有直接移动骨骼
      (`|ExecutionSequence`
        (:`then_0`
          ;;[0.05098 0.05098 0.05098] 移动末端骨骼到目标点
          (bind _returnvalue (`self.LerpEndBonePosition` (`self.Cfg_Free_MoveLerpSpeed`) (`self.Free_LockPosition`)))
          (`ControlRigComponent.SetControlPosition` (`self.ControlRig`) "Bone_002_end_ctrl" _returnvalue "LocalSpace"))
        (:`then_1`
          ;;[0.05098 0.05098 0.05098] 移动根骨骼到目标点
          (bind _returnvalue_2 (`self.LerpRootBonePosition` (`self.Cfg_Free_MoveLerpSpeed`) (`self.Free_MovePosition`)))
          (`self.K2_SetActorLocation` _returnvalue_2))
        (:`then_2`
          ;;[0.05098 0.05098 0.05098] 判断根骨骼是否到达目标点，如果到达则切换锁定骨骼，继续移动
          (if (`self.CheckIsAlreadyMoveToTarget` (`self.K2_GetActorLocation`) (`self.Free_MovePosition`))
            (bind (_lockposition _moveposition) (`self.Change Free Move Lock Bone` false (`self.Free_MoveForwardNormal`) (`self.Cfg_Free_TraceUpOffset`) (`self.Cfg_Free_TraceDownOffset`)))
            (set `self.Free_LockPosition` _lockposition)
            (set `self.Free_MovePosition` _moveposition))))
      (else
        ;[0.05098 0.05098 0.05098] 锁定根骨骼，移动末端骨骼，因为根骨骼跟随actor位置，所以这一步不对根骨骼处理
        (`|ExecutionSequence`
          (:`then_0`
            ;;[0.05098 0.05098 0.05098] 移动末端骨骼到目标点
            (bind _returnvalue_3 (`self.LerpEndBonePosition` (`self.Cfg_Free_MoveLerpSpeed`) (`self.Free_MovePosition`)))
            (`ControlRigComponent.SetControlPosition` (`self.ControlRig`) "Bone_002_end_ctrl" _returnvalue_3 "LocalSpace"))
          (:`then_1`
            ;;[0.05098 0.05098 0.05098] 判断末端骨骼是否到达目标点，如果到达则切换锁定骨骼
            (if (`self.CheckIsAlreadyMoveToTarget` (`SceneComponent.GetSocketLocation` (`self.Leg`) (`self.EndBoneName`)) (`self.Free_MovePosition`))
              (bind (_lockposition_2 _moveposition_2) (`self.Change Free Move Lock Bone` true (`self.Free_MoveForwardNormal`) (`self.Cfg_Free_TraceUpOffset`) (`self.Cfg_Free_TraceDownOffset`)))
              (set `self.Free_LockPosition` _lockposition_2)
              (set `self.Free_MovePosition` _moveposition_2))))))))

(fn `Init Free Move`
  (params (BodyPosition :type "Vector Structure"))
  (`|ExecutionSequence`
    (:`then_0`
      ;[0.05098 0.05098 0.05098] 初始化自由移动
      ;;[0.05098 0.05098 0.05098] 基于根骨骼更新一次Actor位置，避免物理模拟后初始位置错误
      (`self.K2_SetActorLocation` (`SceneComponent.GetSocketLocation` (`self.Leg`) (`self.RootBoneName`))))
    (:`then_1`
      ;;[0.05098 0.05098 0.05098] 根据自身位置及目标位置设置移动方向
      (`self.UpdateFreeMoveDirection`))
    (:`then_2`
      ;;[0.05098 0.05098 0.05098] 更新锁定目标点与移动目标点
      (bind (_lockposition _moveposition) (`self.Change Free Move Lock Bone` false (`self.Free_MoveForwardNormal`) (`self.Cfg_Free_TraceUpOffset`) (`self.Cfg_Free_TraceDownOffset`)))
      (set `self.Free_LockPosition` _lockposition)
      (set `self.Free_MovePosition` _moveposition))
    (:`then_3`
      ;;[0.05098 0.05098 0.05098] 设置移动模式为自由移动
      (`self.ChangeMoveStyle` "NewEnumerator1")
      (set `self.Free_IsFinishMove` false))))

(fn `Init Physic Move`
  (`|ExecutionSequence`
    (:`then_0`
      ;[0 0.3833 1] 初始化物理移动模式
      ;;[1 1 1] 禁用ControlRig
      (`ActorComponent.Deactivate` (`self.ControlRig`)))
    (:`then_1`
      ;;[1 1 1] 开启物理模拟
      (`PrimitiveComponent.SetSimulatePhysics` (`self.Leg`) true)
      (`SkeletalMeshComponent.SetAllBodiesSimulatePhysics` (`self.Leg`) true)
      (`SkeletalMeshComponent.SetAllBodiesPhysicsBlendWeight` (`self.Leg`) 1.0 false)
      (`PrimitiveComponent.AddImpulse` (`self.Leg`) (* (`KismetMathLibrary.MakeVector` (.x (`KismetMathLibrary.RandomUnitVector`)) (.y (`KismetMathLibrary.RandomUnitVector`)) 1.0) 80000) "Bone" false))
    (:`then_2`
      ;;[1 1 1] 解绑Actor，设置移动状态
      (`self.ChangeMoveStyle` "NewEnumerator3"))))

(fn `Init Snap Move`
  (`self.ChangeMoveStyle` "NewEnumerator2"))

(fn `InitBindMoveConfig`
  (bind (_traceoffset _tracedistance _legoverrangedistance _leglerpspeed) (break `/Game/Procedural/GameData/LegBindMoveConfig` (`self.Bind_MoveConfig`)))
  (set `self.Cfg_Bind_TraceOffset` _traceoffset)
  (set `self.Cfg_Bind_TraceDistance` _tracedistance)
  (set `self.Cfg_Bind_LegOverRangeDistance` _legoverrangedistance)
  (set `self.Cfg_Bind_LegLerpSpeed` _leglerpspeed))

(fn `InitFreeMoveConfig`
  (bind (_traceupoffset _tracedownoffset _minmovedistanceratio _maxmovedistanceratio _movelerpspeed) (break `/Game/Procedural/GameData/LegFreeMoveConfig` (`self.Free_MoveConfig`)))
  (set `self.Cfg_Free_TraceUpOffset` _traceupoffset)
  (set `self.Cfg_Free_TraceDownOffset` _tracedownoffset)
  (set `self.Cfg_Free_MinMoveDistanceRatio` _minmovedistanceratio)
  (set `self.Cfg_Free_MaxMoveDistanceRatio` _maxmovedistanceratio)
  (set `self.Cfg_Free_MoveLerpSpeed` _movelerpspeed))

(fn `LerpEndBonePosition`
  (params (LerpSpeed :type "Float (double-precision)") (TargetPosition :type "Vector Structure"))
  (returns (ReturnValue :type "Vector Structure"))
  (return (`KismetMathLibrary.VInterpTo` (`ControlRigComponent.GetControlPosition` (`self.ControlRig`) "Bone_002_end_ctrl" "LocalSpace") (`local.TargetPosition`) (`self.Delta Seconds`) (`local.LerpSpeed`))))

(fn `LerpRootBonePosition`
  (params (LerpSpeed :type "Float (double-precision)") (TargetPosition :type "Vector Structure"))
  (returns (ReturnValue :type "Vector Structure"))
  (return (`KismetMathLibrary.VInterpTo` (`self.K2_GetActorLocation`) (`local.TargetPosition`) (`self.Delta Seconds`) (`local.LerpSpeed`))))

(fn `ReCombineLeg`
  (`self.K2_AttachToComponent` (`Character.Mesh` (`self.ParentReference`)) (`self.BindSocketName`) "SnapToTarget" "KeepRelative" "KeepWorld"))

(fn `UpdateFreeMoveDirection`
  (set `self.Free_MoveForwardNormal` (`KismetMathLibrary.Normal` (- (`SceneComponent.GetSocketLocation` (`Character.Mesh` (`self.ParentReference`)) (`self.BindSocketName`)) (`self.K2_GetActorLocation`)))))

(fn `UserConstructionScript`)
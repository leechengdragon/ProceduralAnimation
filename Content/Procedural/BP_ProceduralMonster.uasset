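; Procedural monster with child-actor legs that can break apart into physics and recombine.
; The construction script gathers AC_Leg child actors under the capsule, giving each a back-reference and its over-range distance from Config.
; BreakLimbs enables physics on every leg and simulates physics on the body mesh.
; LimbsCombine disables leg physics and starts each leg moving to the capsule's location, without turning off mesh simulation.
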(event `self.ReceiveBeginPlay`)

(event `BreakLimbs`
  (`self.ActiveMonsterPhysic`))

(event `LimbsCombine`
  (`self.TriggerLegMoveToBody`))

(fn `ActiveMonsterPhysic`
  (for _array_element (`self.Legs`)
    (`/Game/Procedural/AC_Leg.Active Physic` _array_element)
    (`PrimitiveComponent.SetSimulatePhysics` (`self.Mesh`) true)))

(fn `TriggerLegMoveToBody`
  (for _array_element (`self.Legs`)
    (`/Game/Procedural/AC_Leg.Deactive Physic` _array_element)
    (`/Game/Procedural/AC_Leg.BeginMoveToBody` _array_element (`SceneComponent.K2_GetComponentLocation` (`self.CapsuleComponent`)))))

(fn `UserConstructionScript`
  (for _array_element (`SceneComponent.GetChildrenComponents` (`self.CapsuleComponent`) false)
    (bind _aschild_actor_component (cast `ChildActorComponent` _array_element))
    (bind _asac_leg (cast `/Game/Procedural/AC_Leg` (`ChildActorComponent.ChildActor` _aschild_actor_component)))
    (`KismetArrayLibrary.Array_Add` (`self.Legs`) _asac_leg)
    (set `/Game/Procedural/AC_Leg.Over Range Distance` (`.LegOverRangeDistance_3_027EAFAC458280EED24631B317A111A3` (break `/Game/Procedural/GameData/ProceduralConfig` (`self.Config`))) _asac_leg)
    (set `/Game/Procedural/AC_Leg.ParentReference` self _asac_leg)))